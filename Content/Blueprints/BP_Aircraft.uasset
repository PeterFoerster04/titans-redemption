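; Player aircraft Blueprint that handles engine and crash audio, out-of-bounds respawn, camera shake and pausing.
; Tick drives thruster volume and booster pitch from thrust, gear and boost state, and clears the crash-delay flag after a delay.
; Leaving the map blocks input and fades the camera around a teleport to PlayerStart.
; Static mesh hits play a crash sound, while Enhanced Input toggles the pause menu, cursor and input mode.
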(event OnComponentHit(m_Mesh)
  (params (HitComponent :type Primitive%20Component%20Object%20Reference) (OtherActor :type Actor%20Object%20Reference) (OtherComp :type Primitive%20Component%20Object%20Reference) (NormalImpulse :type Vector :default "0, 0, 0") (Hit :type Hit%20Result%20Structure%20%28by%20ref%29))
  (Utilities|Casting|CastToStaticMeshActor OtherActor)
  (Audio|PlaySoundatLocation "/Game/Audio/MetaSound/Vehicle/MS_Crash.MS_Crash" (Transformation|GetWorldLocation (Variables|Default|GetCrashAudioComponent)) "0, 0, 0" 1.0 1.0 0.0 0 0 0 0))

(event Input|EnhancedActionEvents|EnhancedInputActionIA_Pause
  (params (ActionValue :type Boolean) (ElapsedSeconds :type Float%20%28double-precision%29) (TriggeredSeconds :type Float%20%28double-precision%29) (InputAction :type Input%20Action%20Object%20Reference :default "/Game/Input/Actions/IA_Pause.IA_Pause"))
  (bind _returnvalue (Game|GetPlayerController 0))
  (:Started
    (if (Variables|Default|GetIsInPauseMenu)
      (Variables|Default|SetIsInPauseMenu false)
      (Widget|RemovefromParent (Variables|Default|GetPauseMenu))
      (bind _settingsmenu (Variables|Default|GetSettingsMenu)
        (:then
          (Widget|RemovefromParent _settingsmenu))
        (:else
          _))
      (Game|SetGamePaused false)
      (Variables|/Script/Engine.PlayerController|SetbShowMouseCursor _returnvalue false)
      (Input|SetInputModeGameOnly _returnvalue false)
      (else
        (Variables|Default|SetIsInPauseMenu true)
        (bind _returnvalue_2 (UserInterface|CreateWidget "/Game/Blueprints/BP_Pausemenu.BP_Pausemenu_C"))
        (bind _output_get (Variables|Default|SetPauseMenu _returnvalue_2))
        (UserInterface|Viewport|AddtoViewport _output_get 0)
        (Game|SetGamePaused true)
        (Variables|/Script/Engine.PlayerController|SetbShowMouseCursor _returnvalue true)
        (Input|SetInputModeGameandUI _returnvalue _output_get "DoNotLock" true false)))))

(event EventBeginPlay
  (Audio|Components|Audio|Stop (Variables|Default|GetCrashAudioComponent))
  (Audio|Parameter|SetFloatParameter (Variables|Default|GetThrusterAudioComponent) "SoundMultiplier" 0.05 :!class /Script/Engine.AudioComponent))

(event EventTick
  (params (DeltaSeconds :type Float%20%28single-precision%29))
  (bind _returnvalue (Game|GetPlayerCameraManager 0))
  (bind _self self)
  (bind _thrusterstandardvolume (Variables|Default|GetThrusterStandardVolume))
  (bind _thrusteraudiocomponent (Variables|Default|GetThrusterAudioComponent))
  (bind _m_currentgear (Variables|Default|Getm_CurrentGear))
  (bind _m_maxgear (Variables|Default|Getm_MaxGear))
  (bind _returnvalue_2 (/ _m_currentgear _m_maxgear))
  (bind _returnvalue_3 (* _returnvalue_2 _thrusterstandardvolume))
  (if (> (Variables|Default|Getm_Thrust) 0.0)
    (Audio|Parameter|SetFloatParameter _thrusteraudiocomponent "SoundMultiplier" _returnvalue_3 :!class /Script/Engine.AudioComponent)
    (if (Variables|Default|Getm_Boosting)
      (Audio|Parameter|SetFloatParameter _thrusteraudiocomponent "BoosterPitch" 1e+01 :!class /Script/Engine.AudioComponent)
      (Audio|Parameter|SetFloatParameter _thrusteraudiocomponent "SoundMultiplier" (Variables|Default|GetThrusterBoostVolume) :!class /Script/Engine.AudioComponent)
      (else
        (Audio|Parameter|SetFloatParameter _thrusteraudiocomponent "BoosterPitch" 0.0 :!class /Script/Engine.AudioComponent)
        (Audio|Parameter|SetFloatParameter _thrusteraudiocomponent "SoundMultiplier" _returnvalue_3 :!class /Script/Engine.AudioComponent)))
    (elif (Variables|Default|Getm_InputBlocked)
      (Audio|Parameter|SetFloatParameter _thrusteraudiocomponent "SoundMultiplier" 0.0 :!class /Script/Engine.AudioComponent)
      (else
        (Audio|Parameter|SetFloatParameter _thrusteraudiocomponent "SoundMultiplier" (Variables|Default|GetThrusterIdleVolume) :!class /Script/Engine.AudioComponent))))
  (if (Variables|Default|Getm_PlayerOutOfMapRange)
    (Variables|Default|Setm_InputBlocked true)
    (CameraFades|StartCameraFade :self _returnvalue :ToAlpha 1.0 :Duration 1.5 :bHoldWhenFinished true)
    (bind _returnvalue_4 (Actor|GetActorOfClass "/Script/Engine.PlayerStart"))
    (Utilities|FlowControl|Delay 2.0)
    (Variables|Default|Setm_PlayerOutOfMapRange false)
    (Class|Aircraft|PortPlayerBacktoSpawn (Transformation|GetActorLocation _returnvalue_4))
    (Variables|Default|Setm_InputBlocked false)
    (CameraFades|StartCameraFade :self _returnvalue :FromAlpha 1.0 :Duration 2.0))
  (if (Variables|Default|Getm_IsOnCrashDelay _self)
    (Utilities|FlowControl|Delay 5.0)
    (Variables|Default|Setm_IsOnCrashDelay _self false)))

(event EventExplosionCamShake
  (Camera|PlayWorldCameraShake "/Game/Blueprints/BP_CamShakeAsset.BP_CamShakeAsset_C" (Transformation|GetActorLocation) 0.0 9e+05))

(event Input|KeyboardEvents|1
  (params (Key :type Key%20Structure :default "None"))
  (:Pressed
    (Viewport|RemoveAllWidgets)))

(event Input|KeyboardEvents|2
  (params (Key :type Key%20Structure :default "None")))

(fn ConstructionScript)
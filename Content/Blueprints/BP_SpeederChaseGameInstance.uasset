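; Game instance for Speeder Chase that owns the game's single save object and keeps it for the whole session.
; On Init it loads slot "0" into MSaves, or creates a fresh BP_SpeederSaveGame in memory if none exists.
; SaveSaves writes MSaves back on Shutdown, printing a message on failure.
; ClearSave deletes the slot and reloads, which yields a new empty save.
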(event Custom|Clear%20Save
  (SaveGame|DeleteGameinSlot "0")
  (Class|SpeederChaseGameInstance|LoadSaves))

(event EventShutdown
  (Class|SpeederChaseGameInstance|SaveSaves))

(event EventInit
  (Class|SpeederChaseGameInstance|LoadSaves))

(event EventLoadSaves
  (bind _returnvalue (SaveGame|DoesSaveGameExist "0"))
  (if _returnvalue
    (bind _returnvalue_2 (SaveGame|LoadGamefromSlot "0"))
    (bind _asspeeder_save_game (Utilities|Casting|CastToSpeederSaveGame _returnvalue_2))
    (Variables|Default|Setm_Saves _asspeeder_save_game)
    (else
      (bind _returnvalue_3 (SaveGame|CreateSaveGameObject "/Game/Blueprints/BP_SpeederSaveGame.BP_SpeederSaveGame_C"))
      (Variables|Default|Setm_Saves _returnvalue_3))))

(event EventSaveSaves
  (bind _returnvalue (SaveGame|SaveGametoSlot (Variables|Default|Getm_Saves) "0"))
  (if (not _returnvalue)
    (Development|PrintString "Failed to save game")))
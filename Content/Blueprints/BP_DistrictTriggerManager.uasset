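; Manager actor that briefly shows a district's name on screen when an Aircraft enters one of seven district trigger volumes, including the city center.
; Each trigger's overlap passes its district index to DisplayDistrictName, then removes the returned widget after a two-second delay.
; DisplayDistrictName ignores non-Aircraft actors and VehicleAttachment components, and creates a new DistrictTextWidget per accepted overlap, so its in-viewport check does not prevent duplicates.
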(event OnComponentBeginOverlap(District0CityCenterTrigger)
  (params (OverlappedComponent :type Primitive%20Component%20Object%20Reference) (OtherActor :type Actor%20Object%20Reference) (OtherComp :type Primitive%20Component%20Object%20Reference) (OtherBodyIndex :type Integer) (bFromSweep :type Boolean) (SweepResult :type Hit%20Result%20Structure%20%28by%20ref%29))
  (bind _created_widget (CallFunction|DisplayDistrictName OtherComp 0 OtherActor))
  (Utilities|FlowControl|Delay 2.0)
  (Utilities|IsValid _created_widget
    (:Is%20Valid
      (Widget|RemovefromParent _created_widget))))

(event OnComponentBeginOverlap(District1Trigger)
  (params (OverlappedComponent :type Primitive%20Component%20Object%20Reference) (OtherActor :type Actor%20Object%20Reference) (OtherComp :type Primitive%20Component%20Object%20Reference) (OtherBodyIndex :type Integer) (bFromSweep :type Boolean) (SweepResult :type Hit%20Result%20Structure%20%28by%20ref%29))
  (bind _created_widget (CallFunction|DisplayDistrictName OtherComp 1 OtherActor))
  (Utilities|FlowControl|Delay 2.0)
  (Utilities|IsValid _created_widget
    (:Is%20Valid
      (Widget|RemovefromParent _created_widget))))

(event OnComponentBeginOverlap(District2Trigger)
  (params (OverlappedComponent :type Primitive%20Component%20Object%20Reference) (OtherActor :type Actor%20Object%20Reference) (OtherComp :type Primitive%20Component%20Object%20Reference) (OtherBodyIndex :type Integer) (bFromSweep :type Boolean) (SweepResult :type Hit%20Result%20Structure%20%28by%20ref%29))
  (bind _created_widget (CallFunction|DisplayDistrictName OtherComp 2 OtherActor))
  (Utilities|FlowControl|Delay 2.0)
  (Utilities|IsValid _created_widget
    (:Is%20Valid
      (Widget|RemovefromParent _created_widget))))

(event OnComponentBeginOverlap(District3Trigger)
  (params (OverlappedComponent :type Primitive%20Component%20Object%20Reference) (OtherActor :type Actor%20Object%20Reference) (OtherComp :type Primitive%20Component%20Object%20Reference) (OtherBodyIndex :type Integer) (bFromSweep :type Boolean) (SweepResult :type Hit%20Result%20Structure%20%28by%20ref%29))
  (bind _created_widget (CallFunction|DisplayDistrictName OtherComp 3 OtherActor))
  (Utilities|FlowControl|Delay 2.0)
  (Utilities|IsValid _created_widget
    (:Is%20Valid
      (Widget|RemovefromParent _created_widget))))

(event OnComponentBeginOverlap(District4Trigger)
  (params (OverlappedComponent :type Primitive%20Component%20Object%20Reference) (OtherActor :type Actor%20Object%20Reference) (OtherComp :type Primitive%20Component%20Object%20Reference) (OtherBodyIndex :type Integer) (bFromSweep :type Boolean) (SweepResult :type Hit%20Result%20Structure%20%28by%20ref%29))
  (bind _created_widget (CallFunction|DisplayDistrictName OtherComp 4 OtherActor))
  (Utilities|FlowControl|Delay 2.0)
  (Utilities|IsValid _created_widget
    (:Is%20Valid
      (Widget|RemovefromParent _created_widget))))

(event OnComponentBeginOverlap(District5Trigger)
  (params (OverlappedComponent :type Primitive%20Component%20Object%20Reference) (OtherActor :type Actor%20Object%20Reference) (OtherComp :type Primitive%20Component%20Object%20Reference) (OtherBodyIndex :type Integer) (bFromSweep :type Boolean) (SweepResult :type Hit%20Result%20Structure%20%28by%20ref%29))
  (bind _created_widget (CallFunction|DisplayDistrictName OtherComp 5 OtherActor))
  (Utilities|FlowControl|Delay 2.0)
  (Utilities|IsValid _created_widget
    (:Is%20Valid
      (Widget|RemovefromParent _created_widget))))

(event OnComponentBeginOverlap(District6Trigger)
  (params (OverlappedComponent :type Primitive%20Component%20Object%20Reference) (OtherActor :type Actor%20Object%20Reference) (OtherComp :type Primitive%20Component%20Object%20Reference) (OtherBodyIndex :type Integer) (bFromSweep :type Boolean) (SweepResult :type Hit%20Result%20Structure%20%28by%20ref%29))
  (bind _created_widget (CallFunction|DisplayDistrictName OtherComp 6 OtherActor))
  (Utilities|FlowControl|Delay 2.0)
  (Utilities|IsValid _created_widget
    (:Is%20Valid
      (Widget|RemovefromParent _created_widget))))

(event EventBeginPlay)

(event Collision|EventActorBeginOverlap
  (params (OtherActor :type Actor%20Object%20Reference)))

(event EventTick
  (params (DeltaSeconds :type Float%20%28single-precision%29)))

(fn ConstructionScript)

(fn DisplayDistrictName
  (params (CompTriggered :type Primitive%20Component%20Object%20Reference) (DistrictIndex :type Integer) (ActorTriggered :type Actor%20Object%20Reference))
  (Utilities|Casting|CastToAircraft ActorTriggered)
  (Utilities|Casting|CastToVehicleAttachment CompTriggered
    (:CastFailed
      (bind _returnvalue (UserInterface|CreateWidget (Variables|Default|GetDistrictTextWidget)))
      (if (not (UserInterface|Viewport|IsinViewport _returnvalue))
        (Default|SetDistrictText _returnvalue DistrictIndex)
        (UserInterface|Viewport|AddtoViewport _returnvalue 0)
        (return _returnvalue)))))
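; Crane actor that swings its static mesh back and forth between two target rotations, TargetRot and TargetRot2.
; Each Tick calls RotateTo, which eases relative roll, pitch and yaw with FInterpTo and reports arrival within an error tolerance.
; On arrival, a random Delay holds before the Reverse flag flips to send it toward the other rotation.
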(event EventBeginPlay)

(event Collision|EventActorBeginOverlap
  (params (OtherActor :type Actor%20Object%20Reference)))

(event EventTick
  (params (DeltaSeconds :type Float%20%28single-precision%29))
  (bind _returnvalue (Math|Random|RandomFloatinRange 2.0 2e+01))
  (bind _rotspeed (Variables|Default|GetRotSpeed))
  (if (Variables|Default|GetReverse)
    (bind _finished (CallFunction|Rotateto (Variables|Default|GetTargetRot2) (Variables|Default|GetStaticMesh) 5.0 DeltaSeconds _rotspeed))
    (if _finished
      (Utilities|FlowControl|Delay _returnvalue)
      (Variables|Default|SetReverse false))
    (else
      (bind _finished_2 (CallFunction|Rotateto (Variables|Default|GetTargetRot) (Variables|Default|GetStaticMesh) 5.0 DeltaSeconds _rotspeed))
      (if _finished_2
        (Utilities|FlowControl|Delay _returnvalue)
        (Variables|Default|SetReverse true)))))

(fn ConstructionScript)

(fn Rotateto
  (params (Rotator :type Rotator) (Static%20Mesh :type Static%20Mesh%20Component%20Object%20Reference) (RotateErrorTolerance :type Float%20%28double-precision%29) (DeltaTime :type Float%20%28double-precision%29) (Speed :type Float%20%28double-precision%29))
  (bind (_roll _pitch _yaw) (Math|Rotator|BreakRotator Rotator))
  (bind _relativerotation (Variables|/Script/Engine.SceneComponent|GetRelativeRotation Static%20Mesh))
  (bind (_roll_2 _pitch_2 _yaw_2) (Math|Rotator|BreakRotator _relativerotation))
  (Transformation|SetRelativeRotation Static%20Mesh (Math|Rotator|MakeRotator (Math|Interpolation|FInterpTo _roll_2 _roll DeltaTime Speed) (Math|Interpolation|FInterpTo _pitch_2 _pitch DeltaTime Speed) (Math|Interpolation|FInterpTo _yaw_2 _yaw DeltaTime Speed)) false false)
  (if (Utilities|Operators|EqualEqual _relativerotation Rotator RotateErrorTolerance)
    (return true)
    (else
      (return false))))
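; BP_Criminal is a criminal actor with an on-screen marker and music that grows louder as the player's aircraft gets closer.
; BeginPlay caches the marker widget and the player aircraft's mesh, then starts the sound player silent.
; Each Tick feeds the marker's world location to the widget and turns the clamped distance to the player into the DistanceMultiplier sound parameter, which drops to zero while the criminal is flagged as EMP'd.
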(event EventBeginPlay
  (bind _criminalsoundplayer (Variables|Default|GetCriminalSoundPlayer))
  (bind _asbp_criminal_marker (Utilities|Casting|CastToBP_CriminalMarker (UserInterface|GetWidget (Variables|Default|Getm_Marker))))
  (Variables|Default|SetMarkerWidget _asbp_criminal_marker)
  (Audio|Parameter|SetFloatParameter _criminalsoundplayer "DistanceMultiplier" 0.0 :!class /Script/Engine.AudioComponent)
  (Audio|Components|Audio|Play _criminalsoundplayer 0.0)
  (bind _asaircraft (Utilities|Casting|CastToAircraft (Game|Player|GetPlayerPawn 0)))
  (Variables|Default|SetPlayerMesh (Actor|GetComponentbyClass _asaircraft "/Script/Engine.MeshComponent")))

(event Collision|EventActorBeginOverlap
  (params (OtherActor :type Actor%20Object%20Reference)))

(event EventTick
  (params (DeltaSeconds :type Float%20%28single-precision%29))
  (bind _musicmaxdistvolume (Variables|Default|GetMusicMaxDistVolume))
  (bind _criminalsoundplayer (Variables|Default|GetCriminalSoundPlayer))
  (bind _output_get (Variables|/Game/Blueprints/BP_CriminalMarker.BP_CriminalMarker_C|SetMarkerLocation (Variables|Default|GetMarkerWidget) (Transformation|GetWorldLocation (Variables|Default|Getm_Marker))))
  (if (Variables|Default|Getm_WasEMPd)
    (Audio|Parameter|SetFloatParameter _criminalsoundplayer "DistanceMultiplier" 0.0 :!class /Script/Engine.AudioComponent)
    (else
      (Audio|Parameter|SetFloatParameter _criminalsoundplayer "DistanceMultiplier" (- 1.0 (/ (Math|Float|Clamp(Float) (/ (Math|Float|Absolute(Float) (Math|Vector|VectorLength (- _output_get (Transformation|GetWorldLocation (Variables|Default|GetPlayerMesh))))) 1e+02) (Variables|Default|GetMusicMinDistVolume) _musicmaxdistvolume) _musicmaxdistvolume)) :!class /Script/Engine.AudioComponent))))

(fn ConstructionScript)
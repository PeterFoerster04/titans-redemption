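; Ambient sound manager that switches audio between inside and outside states based on whether the player is in the police station's garage.
; On BeginPlay it finds the PoliceStation actor and starts its Audio component.
; Tick polls the station's MPLayerIsInGarage flag and fires PlayerInside or PlayerOutside trigger parameters on the audio.
; Two DoOnce nodes reset each other, so each trigger fires only when the state changes.
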(event EventBeginPlay
  (bind _returnvalue (Actor|GetActorOfClass "/Script/SpeederGame.PoliceStation"))
  (Variables|Default|SetPolice _returnvalue)
  (Audio|Components|Audio|Play (Variables|Default|GetAudio) 0.0))

(event Collision|EventActorBeginOverlap
  (params (OtherActor :type Actor%20Object%20Reference)))

(event EventTick
  (params (DeltaSeconds :type Float%20%28single-precision%29))
  (bind _audio (Variables|Default|GetAudio))
  (if (Variables|/Script/SpeederGame.PoliceStation|Getm_PLayerIsInGarage (Variables|Default|GetPolice))
    (Utilities|FlowControl|DoOnce false :!label _label
      (:Completed
        (Class|AudioParameterControllerInterface|SetTriggerParameter _audio "PlayerInside")
        (goto _label_2 Reset)))
    (else
      (Utilities|FlowControl|DoOnce false :!label _label_2
        (:Completed
          (Class|AudioParameterControllerInterface|SetTriggerParameter _audio "PlayerOutside")
          (goto _label Reset))))))

(fn ConstructionScript)
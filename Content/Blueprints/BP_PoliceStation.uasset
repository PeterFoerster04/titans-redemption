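; Police station Blueprint that presents mission results and feeds its world location to a police marker widget every tick.
; ShowWinScreen fades the camera, plays a jail-bars sound, then uses timed delays to reveal up to three stars from the absolved-to-initial time ratio, plus reward and bonus.
; ShowFailScreen briefly shows the failure reason with a sound.
; ChangeVehicleThrusterVolume is empty, leaving its aircraft audio logic unconnected.
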(event EventBeginPlay
  (bind _asbp_police_marker (Utilities|Casting|CastToBP_PoliceMarker (UserInterface|GetWidget (Variables|Default|GetMarker))))
  (Variables|Default|SetMarkerWidget _asbp_police_marker))

(event EventTick
  (params (DeltaSeconds :type Float%20%28single-precision%29))
  (bind _markerwidget (Variables|Default|GetMarkerWidget)
    (:then
      (Variables|/Game/Blueprints/BP_PoliceMarker.BP_PoliceMarker_C|SetMarkerLocation _markerwidget (Transformation|GetWorldLocation (Variables|Default|GetMarker))))
    (:else)))

(event EventShowWinScreen
  (bind _returnvalue (Game|GetPlayerCameraManager 0))
  (bind _self self)
  (bind _self_2 self)
  (bind _m_missionabsolvedtime (Variables|Default|Getm_MissionAbsolvedTime _self_2))
  (bind _m_missioninitialtime (Variables|Default|Getm_MissionInitialTime _self_2))
  (bind _returnvalue_2 (/ _m_missionabsolvedtime _m_missioninitialtime))
  (bind _m_currentmission (Variables|Default|Getm_CurrentMission _self_2)
    (:then
      (if (Variables|/Script/SpeederGame.CaseMission|Getm_MissionWasAbsolved _m_currentmission)
        (bind _m_winscreen (Variables|/Script/SpeederGame.PoliceStationUIManager|Getm_WinScreen (Variables|Default|Getm_PoliceUIManager _self_2))
          (:then
            (bind _returnvalue_3 (UserInterface|CreateWidget _m_winscreen))
            (bind _asbp_win_screen (Utilities|Casting|CastToBP_WinScreen _returnvalue_3))
            (CameraFades|StartCameraFade :self _returnvalue :ToAlpha 1.0 :Duration 1.5 :bHoldWhenFinished true)
            (Utilities|FlowControl|Delay 1.0)
            (Audio|PlaySound2D "/Game/Audio/Assets/UI/CriminalBarsSound.CriminalBarsSound" 1.0 1.0 0.0 0 0)
            (Utilities|FlowControl|Delay 0.5)
            (if (not (UserInterface|Viewport|IsinViewport _asbp_win_screen))
              (UserInterface|Viewport|AddtoViewport _asbp_win_screen 1)
              (CameraFades|StartCameraFade :self _returnvalue :FromAlpha 1.0 :Duration 1.5)
              (if (> _returnvalue_2 0.2)
                (Utilities|FlowControl|Delay 1.0)
                (Default|ActivateSpecificStar _asbp_win_screen 1)
                (if (> _returnvalue_2 0.5)
                  (Utilities|FlowControl|Delay 1.0)
                  (Default|ActivateSpecificStar _asbp_win_screen 2)
                  (if (> _returnvalue_2 0.7)
                    (Utilities|FlowControl|Delay 1.8)
                    (Default|ActivateSpecificStar _asbp_win_screen 3))))
              (Utilities|FlowControl|Delay 0.5)
              (Default|SetRewardText _asbp_win_screen (Math|Float|Truncate (Variables|Default|Getm_BaseRewardForAbsolvedMission _self)))
              (Utilities|FlowControl|Delay 1.0)
              (Default|SetBonusText _asbp_win_screen (Math|Float|Truncate (Variables|Default|Getm_TimeBonusReward _self)))
              (Utilities|FlowControl|Delay 2.0)
              (Widget|RemovefromParent _asbp_win_screen)))
          (:else))))
    (:else)))

(event EventShowFailScreen
  (params (a_ReasonWasTime :type Boolean))
  (bind _m_failscreen (Variables|/Script/SpeederGame.PoliceStationUIManager|Getm_FailScreen (Variables|Default|Getm_PoliceUIManager self))
    (:then
      (bind _returnvalue (UserInterface|CreateWidget _m_failscreen))
      (bind _asbp_mission_fail_screen (Utilities|Casting|CastToBP_MissionFailScreen _returnvalue))
      (Default|SetFailReasonText _asbp_mission_fail_screen a_ReasonWasTime)
      (UserInterface|Viewport|AddtoViewport _asbp_mission_fail_screen 0)
      (Audio|PlaySound2D "/Game/Audio/Assets/UI/MissionFailedSound.MissionFailedSound" 1.0 1.0 0.0 0 0)
      (Utilities|FlowControl|Delay 3.0)
      (Widget|RemovefromParent _asbp_mission_fail_screen))
    (:else)))

(event EventChangeVehicleThrusterVolume
  (params (a_TurnOfVolume :type Boolean) (m_Vehicle :type Aircraft%20Object%20Reference)))

(fn ConstructionScript)
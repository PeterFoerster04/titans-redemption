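; BP_AchievementManager is an actor that unlocks two platform achievements, First Catch and Three Star, through custom events.
; Each event calls ActivateSpecificAchievement, which, despite its name, only checks whether the local player's cached progress for that ID is above zero.
; If it is not, the event writes achievement progress for player controller 0.
; The file only reads the achievement cache and never populates it.
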(event EventBeginPlay)

(event Collision|EventActorBeginOverlap
  (params (OtherActor :type Actor%20Object%20Reference)))

(event EventTick
  (params (DeltaSeconds :type Float%20%28single-precision%29)))

(event EventActivateFirstCatchAchievement
  (bind _firstcatchid (Variables|Default|GetFirstCatchID))
  (bind _wasactivated (CallFunction|ActivateSpecificAchievement _firstcatchid))
  (if (not _wasactivated)
    (|WriteAchievementProgress (Game|GetPlayerController 0) _firstcatchid 1e+02)))

(event EventActivateThreeStarAchievement
  (bind _threestarid (Variables|Default|GetThreeStarID))
  (bind _wasactivated (CallFunction|ActivateSpecificAchievement _threestarid))
  (if (not _wasactivated)
    (|WriteAchievementProgress (Game|GetPlayerController 0) _threestarid 1e+02)))

(fn ConstructionScript)

(fn ActivateSpecificAchievement
  (params (ID :type Name))
  (bind (_bfoundid _progress) (Class|AchievementBlueprintLibrary|GetCachedAchievementProgress (Game|GetPlayerController 0) ID))
  (if _bfoundid
    (return (> _progress 0.0))))
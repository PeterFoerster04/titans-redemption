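; Construction-script Blueprint that tiles a static mesh along a spline as spline mesh components, likely for roads or similar level dressing.
; It can rebuild its spline from a point range on another actor's spline, offset to either side.
; Mesh count and stretch derive from mesh length, end offsets and allowed scale fluctuation, with gap adjustment for closed loops.
; Optional line traces snap spline points to the ground before meshes spawn.
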(fn ConstructionScript
  (bind _splined_mesh (Variables|Default|GetSplined%20Mesh))
  (bind _allowable_scale_fluctuation (Variables|Default|GetAllowable%20Scale%20Fluctuation))
  (bind _actor_with_spline (Variables|SnapSplinetootherSpline|GetActor%20with%20Spline))
  (bind _spline (Variables|Default|GetSpline))
  (bind _spline_2 (Variables|Default|GetSpline))
  (bind _spline_3 (Variables|Default|GetSpline))
  (bind _distance_from_spline (Variables|SnapSplinetootherSpline|GetDistance%20From%20Spline))
  (bind _returnvalue (Actor|GetComponentsByClass _actor_with_spline "/Script/Engine.SplineComponent"))
  (bind _returnvalue_2 (StaticMesh|GetBoundingBox _splined_mesh))
  (bind _returnvalue_3 (- 1.0 _allowable_scale_fluctuation))
  (bind (_min _max) (Utilities|Struct|BreakBox _returnvalue_2))
  (bind _returnvalue_4 (Utilities|Array|Length _returnvalue))
  (bind _output (Utilities|Array|Get(acopy) _returnvalue))
  (if (Variables|Default|GetClosed%20Loop)
    (Spline|SetClosedLoop _spline true true)
    (else
      (Spline|SetClosedLoop _spline false true)))
  ;[1 1 1] Spawns splined mesh along another spline if enabled
  (Utilities|IsValid (Variables|SnapSplinetootherSpline|GetActor%20with%20Spline)
    (:Is%20Valid
      (Variables|/Script/Engine.SplineComponent|SetbInputSplinePointsToConstructionScript (Variables|Default|GetSpline) true)
      (if (== _returnvalue_4 1)
        (LocalVariables|SetActor's%20Spline%20Component (Actor|GetComponentbyClass (Variables|SnapSplinetootherSpline|GetActor%20with%20Spline) "/Script/Engine.SplineComponent"))
        (Utilities|IsValid (LocalVariables|GetActor's%20Spline%20Component) :!label _label
          (:Is%20Valid
            (if (> (Spline|GetNumberOfSplinePoints (LocalVariables|GetActor's%20Spline%20Component)) 1)
              (if (< (Variables|SnapSplinetootherSpline|GetEnd%20Spline%20Point) (- (Spline|GetNumberOfSplinePoints (LocalVariables|GetActor's%20Spline%20Component)) 1))
                _
                (else
                  (Variables|SnapSplinetootherSpline|SetEnd%20Spline%20Point (- (Spline|GetNumberOfSplinePoints (LocalVariables|GetActor's%20Spline%20Component)) 1))))
              (Spline|ClearSplinePoints (Variables|Default|GetSpline) true)
              (if (Variables|SnapSplinetootherSpline|GetLeft%20Side)
                (LocalVariables|SetRight%20Side%20Multiplier -1)
                (LocalVariables|SetTemp%20Spline%20Point (Variables|SnapSplinetootherSpline|GetStart%20Spline%20Point))
                (else
                  (LocalVariables|SetRight%20Side%20Multiplier 1)
                  (LocalVariables|SetTemp%20Spline%20Point (Variables|SnapSplinetootherSpline|GetEnd%20Spline%20Point))))
              (while (and (>= (LocalVariables|GetTemp%20Spline%20Point) (Variables|SnapSplinetootherSpline|GetStart%20Spline%20Point)) (<= (LocalVariables|GetTemp%20Spline%20Point) (Variables|SnapSplinetootherSpline|GetEnd%20Spline%20Point)))
                (Spline|AddSplinePoint (Variables|Default|GetSpline) (Math|Vector|MakeVector (- (.x (Spline|GetLocationatSplinePoint (LocalVariables|GetActor's%20Spline%20Component) (LocalVariables|GetTemp%20Spline%20Point) "World")) (* (Math|Trig|Sin(Degrees) (.yaw (Spline|GetRotationatSplinePoint (LocalVariables|GetActor's%20Spline%20Component) (LocalVariables|GetTemp%20Spline%20Point) "World"))) _distance_from_spline (LocalVariables|GetRight%20Side%20Multiplier))) (+ (.y (Spline|GetLocationatSplinePoint (LocalVariables|GetActor's%20Spline%20Component) (LocalVariables|GetTemp%20Spline%20Point) "World")) (* (Math|Trig|Cos(Degrees) (.yaw (Spline|GetRotationatSplinePoint (LocalVariables|GetActor's%20Spline%20Component) (LocalVariables|GetTemp%20Spline%20Point) "World"))) _distance_from_spline (LocalVariables|GetRight%20Side%20Multiplier))) (.z (Spline|GetLocationatSplinePoint (LocalVariables|GetActor's%20Spline%20Component) (LocalVariables|GetTemp%20Spline%20Point) "World"))) "World" true)
                (if (Variables|SnapSplinetootherSpline|GetLeft%20Side)
                  (Math|Integer|IncrementInt (LocalVariables|GetTemp%20Spline%20Point))
                  (else
                    (Math|Integer|DecrementInt (LocalVariables|GetTemp%20Spline%20Point)))))
              (LocalVariables|SetAlong%20Spline true)
              (for _index (range 0 (- (Spline|GetNumberOfSplinePoints (Variables|Default|GetSpline)) 1))
                (Spline|SetTangentatSplinePoint _spline_2 _index (* (Spline|GetTangentatSplinePoint _spline_2 _index "World") (Variables|Default|GetCurve%20Scale)) "World" true))
              (else
                (LocalVariables|SetAlong%20Spline false :!label _label_2))))
          (:Is%20Not%20Valid
            (goto _label_2)))
        (elif (== _returnvalue_4 0)
          (goto _label_2)
          (else
            (for _array_element _returnvalue
              (if (Utilities|Enum|Equal(Enum) (Utilities|GetObjectName _array_element) (Variables|SnapSplinetootherSpline|GetSpline%20Name))
                (LocalVariables|SetActor's%20Spline%20Component _array_element)
                (LocalVariables|SetName%20Found true)))
            (if (LocalVariables|GetName%20Found)
              (LocalVariables|SetName%20Found false)
              (else
                (Variables|SnapSplinetootherSpline|SetSpline%20Name (Utilities|GetObjectName _output))
                (LocalVariables|SetActor's%20Spline%20Component _output)))
            (Utilities|IsValid (Variables|SnapSplinetootherSpline|GetActor%20with%20Spline)
              (:Is%20Valid
                (goto _label))
              (:Is%20Not%20Valid
                _))))))
    (:Is%20Not%20Valid
      (goto _label_2)))
  (Variables|Default|SetStart%20Offset (|ClampStartOffset))
  (Variables|Default|SetEnd%20Offset (|ClampEndOffset))
  ;[1 1 1] Caclulate number of instances, instance spacing and other math needed to spawn instances
  (if (not (Variables|Default|GetDisable%20Mesh))
    (Variables|Default|GetSplined%20Mesh
      (:then
        (bind _output_get (Variables|Default|SetSpacing (+ (.x (- _max _min)) (Variables|Default|GetOffset))))
        (bind _output_get_2 (Variables|Default|SetNumber%20of%20Instances (Math|Float|Round (/ (- (- (Spline|GetSplineLength (Variables|Default|GetSpline)) (Variables|Default|GetStart%20Offset)) (Variables|Default|GetEnd%20Offset)) _output_get))))
        (Variables|Default|SetIdeal%20Number%20of%20Instances _output_get_2)
        (if (!= (Math|Float|Round (/ (- (- (Spline|GetSplineLength (Variables|Default|GetSpline)) (Variables|Default|GetStart%20Offset)) (Variables|Default|GetEnd%20Offset)) _output_get)) 0)
          (LocalVariables|SetStretch%20Size (/ (/ (- (- (Spline|GetSplineLength (Variables|Default|GetSpline)) (Variables|Default|GetStart%20Offset)) (Variables|Default|GetEnd%20Offset)) _output_get) (Variables|Default|GetNumber%20of%20Instances)))
          (if (not (< (/ (- (- (Spline|GetSplineLength (Variables|Default|GetSpline)) (Variables|Default|GetStart%20Offset)) (Variables|Default|GetEnd%20Offset)) _output_get) (* _returnvalue_3 (Variables|Default|GetNumber%20of%20Instances))))
            _
            (else
              (bind _output_get_3 (Variables|Default|SetNumber%20of%20Instances (- _output_get_2 1))))))
        (if (!= _output_get_3 0)
          (if (> (/ (- (- (Spline|GetSplineLength (Variables|Default|GetSpline)) (Variables|Default|GetStart%20Offset)) (Variables|Default|GetEnd%20Offset)) _output_get) (* (+ _allowable_scale_fluctuation 1.0) (Variables|Default|GetNumber%20of%20Instances)))
            (Variables|Default|SetIdeal%20Stretch%20Size (LocalVariables|GetStretch%20Size))
            (LocalVariables|SetStretch%20Size (/ (* (+ _allowable_scale_fluctuation 1.0) (Variables|Default|GetNumber%20of%20Instances)) (Variables|Default|GetNumber%20of%20Instances)))
            (else
              (Variables|Default|SetIdeal%20Stretch%20Size (LocalVariables|GetStretch%20Size) :!label _label_3)))
          (CallFunction|SnapRoadtoGround (Variables|Default|GetDisable%20Ground%20Snapping)) ; Snap instance to ground if enabled
          ;[1 1 1] Spawn all instances with location and tangents specified
          (if (Variables|Default|GetClosed%20Loop)
            (LocalVariables|SetGap%20Adjustment (|CalculateGapAdjustment (LocalVariables|GetStretch%20Size)))
            (else
              (LocalVariables|SetGap%20Adjustment 0.0)))
          (for _index_2 (range 0 (- (Variables|Default|GetNumber%20of%20Instances) 1))
            (bind _returnvalue_5 (AddComponent|AddSplineMeshComponent false))
            (Components|StaticMesh|SetStaticMesh _returnvalue_5 (Variables|Default|GetSplined%20Mesh))
            (Collision|SetCollisionEnabled _returnvalue_5 "QueryAndPhysics")
            (SplineMesh|SetForwardAxis _returnvalue_5 "X" true)
            (SplineMesh|SetStartandEnd _returnvalue_5 (+ (Spline|GetLocationatDistanceAlongSpline _spline_3 (Math|Float|Max(Float) (+ (- (* _index_2 (* (Variables|Default|GetSpacing) (LocalVariables|GetStretch%20Size))) (Variables|Default|GetOverlap)) (Variables|Default|GetStart%20Offset)) 0.0) "Local") (Math|Vector|MakeVector 0.0 0.0 (Variables|Default|GetMesh%20Vertical%20Offset))) (Math|Vector|ClampVectorSize (Spline|GetTangentatDistanceAlongSpline _spline_3 (Math|Float|Max(Float) (+ (- (* _index_2 (* (Variables|Default|GetSpacing) (LocalVariables|GetStretch%20Size))) (Variables|Default|GetOverlap)) (Variables|Default|GetStart%20Offset)) 0.0) "Local") 0.0 (Variables|Default|GetSpacing)) (+ (Spline|GetLocationatDistanceAlongSpline _spline_3 (+ (* (+ _index_2 1) (+ (* (Variables|Default|GetSpacing) (LocalVariables|GetStretch%20Size)) (LocalVariables|GetGap%20Adjustment))) (Variables|Default|GetStart%20Offset)) "Local") (Math|Vector|MakeVector 0.0 0.0 (Variables|Default|GetMesh%20Vertical%20Offset))) (Math|Vector|ClampVectorSize (Spline|GetTangentatDistanceAlongSpline _spline_3 (+ (* (+ _index_2 1) (+ (* (Variables|Default|GetSpacing) (LocalVariables|GetStretch%20Size)) (LocalVariables|GetGap%20Adjustment))) (Variables|Default|GetStart%20Offset)) "Local") 0.0 (Variables|Default|GetSpacing)) true :!class /Script/Engine.SplineMeshComponent))
          (elif (< _returnvalue_3 (/ (- (- (Spline|GetSplineLength (Variables|Default|GetSpline)) (Variables|Default|GetStart%20Offset)) (Variables|Default|GetEnd%20Offset)) _output_get))
            (LocalVariables|SetStretch%20Size (/ (- (- (Spline|GetSplineLength (Variables|Default|GetSpline)) (Variables|Default|GetStart%20Offset)) (Variables|Default|GetEnd%20Offset)) _output_get))
            (Variables|Default|SetNumber%20of%20Instances 1)
            (goto _label_3)
            (else
              (Development|PrintString "Not enough room for object to be placed")))))
      (:else))))

(fn SnapRoadtoGround
  (params (Disable? :type Boolean))
  (bind _returnvalue (Transformation|GetActorLocation))
  ;[1 1 1] Snap spline to ground
  (if (not Disable?)
    (for _index (range 0 (- (Spline|GetNumberOfSplinePoints (Variables|Default|GetSpline)) 1))
      (bind _outhit (Collision|LineTraceByChannel (Math|Vector|MakeVector (.x (Spline|GetLocationatSplinePoint (Variables|Default|GetSpline) _index "World")) (.y (Spline|GetLocationatSplinePoint (Variables|Default|GetSpline) _index "World")) (+ (.z _returnvalue) 1e+04)) (Math|Vector|MakeVector (.x (Spline|GetLocationatSplinePoint (Variables|Default|GetSpline) _index "World")) (.y (Spline|GetLocationatSplinePoint (Variables|Default|GetSpline) _index "World")) (- (.z _returnvalue) 1e+04)) "TraceTypeQuery1" true (Variables|Default|GetActors%20to%20Ignore%20when%20Snapping%20to%20Ground) "None" true "(R=1.000000,G=0.000000,B=0.000000,A=0.000000)"))
      (Spline|SetLocationatSplinePoint (Variables|Default|GetSpline) _index (Math|Vector|MakeVector (.x (Spline|GetLocationatSplinePoint (Variables|Default|GetSpline) _index "World")) (.y (Spline|GetLocationatSplinePoint (Variables|Default|GetSpline) _index "World")) (.z (.ImpactPoint (Collision|BreakHitResult _outhit)))) "World" true))
    (return)
    (else
      (return))))